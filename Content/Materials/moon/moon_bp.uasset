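; Moon Blueprint actor that orbits a Center point by spinning around it.
; On BeginPlay it saves its placed location, moves the actor origin to Center, then puts the Sphere component back at the saved location as an offset.
; Tick increases the actor's yaw at a constant rate scaled by delta time, so the offset sphere circles the center without any explicit orbit math.
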(event EventBeginPlay
  (Variables|Default|Setinitial%20planet%20location (Transformation|GetActorLocation))
  (Transformation|SetActorLocation (Variables|Default|Getcenter) false false)
  (Transformation|SetWorldLocation (Variables|Default|GetSphere) (Variables|Default|Getinitial%20planet%20location) false false))

(event Collision|EventActorBeginOverlap
  (params (OtherActor :type Actor%20Object%20Reference)))

(event EventTick
  (params (DeltaSeconds :type Float%20%28single-precision%29))
  (Transformation|SetActorRotation (Math|Rotator|MakeRotator 0.0 0.0 (+ (.yaw (Transformation|GetActorRotation)) (* DeltaSeconds 1e+01)))))

(fn ConstructionScript)